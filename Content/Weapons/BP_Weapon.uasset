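; Base weapon Blueprint that supplies shared equip, attach and action-montage logic, with empty hooks for equip start, actions and skills.
; On BeginPlay it caches its owning Character and gathers ActionTable rows matching its WeaponType into ActionData.
; PlayAction plays the indexed entry's montage on the owner and sends that entry's Movable setting through SetWeaponMovableMessage.
; EndEquip and Unequip toggle the Equipped flag, and a helper attaches the weapon to a named socket on the owner's mesh.
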(event `self.ReceiveBeginPlay`
  (bind _actiontable (`self.ActionTable`))
  (bind _ascharacter (cast `Character` (`self.GetOwner`)))
  (set `self.OwnerCharacter` _ascharacter)
  (bind _outrownames (`DataTableFunctionLibrary.GetDataTableRowNames` _actiontable))
  (for _array_element _outrownames
    (bind _returnvalue (`|GetDataTableRow` _actiontable _array_element)
      (:`then`
        (if (`|EnumEquality` (`.WeaponType_12_412C723D4BE930FCCBFDF485168EDB5D` (break `/Game/Structures/FAction` _returnvalue)) (`self.WeaponType`))
          (`KismetArrayLibrary.Array_AddUnique` (`self.ActionData`) _returnvalue))))))

(fn `Attach to Owner Character`
  (params (InSocketName :type Name))
  (`self.K2_AttachToComponent` (`Character.Mesh` (`self.OwnerCharacter`)) InSocketName "KeepRelative" "KeepRelative" "KeepRelative"))

(fn `Begin Do Action`)

(fn `BeginEquip`)

(fn `DoAction`)

(fn `DoPressedSkill`)

(fn `DoReleasedSkill`)

(fn `DoSkill`)

(fn `EndDoAction`)

(fn `EndEquip`
  (set `self.Equipped` true))

(fn `PlayAction`
  (params (InIndex :type Integer))
  (bind _ownercharacter (`self.OwnerCharacter`))
  (bind ((`Montage_7_7C6EDC8046AF68AF87DB68A79B562166` _montage) (`PlayRate_23_8167CBB7467E3DFF8ED360B68F80CC27` _playrate) (`Movable_25_4856289E4862D18FF3A8F88A8A05B9A9` _movable)) (break `/Game/Structures/FAction` (`|GetArrayItem` (`self.ActionData`) InIndex)))
  (`Character.PlayAnimMontage` _ownercharacter _montage _playrate "None")
  (message `/Game/Interfaces/IWeapon.SetWeaponMovable` _ownercharacter _movable))

(fn `Unequip`
  (set `self.Equipped` false))

(fn `UserConstructionScript`)