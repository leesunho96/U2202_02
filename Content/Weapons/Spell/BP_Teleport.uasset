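; Teleport spell weapon that moves its owner to the world-static surface point under the cursor.
; While equipped, Tick places a decal on that point aligned to the surface normal, hiding it otherwise.
; DoAction stores a destination offset along the normal, checks and changes owner state via IState, then plays the action with an attached particle effect.
; BeginDoAction relocates the owner without sweep; EndDoAction restores state and re-enables movement via IWeapon.
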(event `self.ReceiveBeginPlay`
  (`parent.ReceiveBeginPlay`)
  (`SceneComponent.SetVisibility` (`self.Decal`) false false))

(event `self.ReceiveTick`
  (params (DeltaSeconds :type "Float (single-precision)"))
  (bind (_outhitresult _outhitlocation _out_hit_normal) (`self.Get Whether Cursor Hits`))
  (bind _decal (`self.Decal`))
  (if (`self.Equipped`)
    (if _outhitresult
      (`SceneComponent.SetVisibility` _decal true false)
      (`SceneComponent.K2_SetWorldLocationAndRotation` _decal _outhitlocation (`KismetMathLibrary.Conv_VectorToRotator` _out_hit_normal) false false)
      (else
        (`SceneComponent.SetVisibility` _decal false false :!label _label)))
    (else
      (goto _label))))

(fn `Begin Do Action`
  (`parent.Begin Do Action`)
  (`self.K2_SetActorLocation` (`self.OwnerCharacter`) (`self.Destination`) false false))

(fn `DoAction`
  (bind (_outhitresult _outhitlocation _out_hit_normal) (`self.Get Whether Cursor Hits`))
  (bind (_particlesystem _transform) (break `/Game/Structures/FEffect` (`.Effect_35_0FBB043C4820649C4A3CA79825DA37BA` (break `/Game/Structures/FAction` (`|GetArrayItem` (`self.ActionData`))))))
  (`parent.DoAction`)
  (if _outhitresult
    (set `self.Destination` (+ _outhitlocation (* _out_hit_normal 100.0)))
    (bind _outobject (`/Game/MacroLibraries/ML_ObjectVerifier.VerifyImplementation` (`self.OwnerCharacter`) "/Game/Interfaces/IState.IState_C")
      (:`True`
        (bind _outresult (message `/Game/Interfaces/IState.IsState` _outobject "NewEnumerator0"))
        (if _outresult
          (message `/Game/Interfaces/IState.SetState` _outobject "NewEnumerator2")
          (`self.PlayAction` 0)
          (`GameplayStatics.SpawnEmitterAttached` _particlesystem (`Character.Mesh` (`self.OwnerCharacter`)) "root" (.location _transform) (.rotation _transform) (.scale _transform) "KeepRelativeOffset" false "AutoRelease"))))))

(fn `EndDoAction`
  (bind _ownercharacter (`self.OwnerCharacter`))
  (`parent.EndDoAction`)
  (message `/Game/Interfaces/IState.SetState` _ownercharacter "NewEnumerator0")
  (bind _outobject (`/Game/MacroLibraries/ML_ObjectVerifier.VerifyImplementation` _ownercharacter "/Game/Interfaces/IWeapon.IWeapon_C")
    (:`True`
      (message `/Game/Interfaces/IWeapon.SetWeaponMovable` _outobject true))))

(fn `Get Whether Cursor Hits`
  (returns (OutHitResult :type Boolean) (OutHitLocation :type "Vector Structure") (`Out Hit Normal` :type "Vector Structure"))
  (bind (_hitresult _returnvalue) (`PlayerController.GetHitResultUnderCursorForObjects` (`GameplayStatics.GetPlayerController` 0) (`|MakeArray` "ObjectTypeQuery1" :!type "EObjectTypeQuery Enum") false))
  (return _returnvalue (`.Location` (`GameplayStatics.BreakHitResult` _hitresult)) (`.Normal` (`GameplayStatics.BreakHitResult` _hitresult))))

(fn `UserConstructionScript`
  (`parent.UserConstructionScript`))