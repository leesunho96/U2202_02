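; Fire storm spell that orbits its owner and periodically damages other characters inside it.
; DoAction checks and sets the owner's state before playing the action, and EndDoAction restores state and weapon movement.
; BeginDoAction attaches the particle to the collision box, randomizes the starting angle and starts damage and duration timers.
; Tick moves the actor around the owner while the particle lives, overlap events track victims, and DestroyStorm cleans up.
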(event `self.ReceiveActorBeginOverlap`
  (params (OtherActor :type "Actor Object Reference"))
  ;[1 1 1] Dagege 판정 위해 겹쳐있는 Enemy들 OverlapedDamagedActor 저장
  (bind _ascharacter (cast `Character` OtherActor))
  (if (!= _ascharacter (`self.OwnerCharacter`))
    (`KismetArrayLibrary.Array_AddUnique` (`self.OverlapedDamegedActors`) _ascharacter)))

(event `self.ReceiveActorEndOverlap`
  (params (OtherActor :type "Actor Object Reference"))
  ;[1 1 1] Dagege 판정 위해 겹쳐있는 Enemy들 OverlapedDamagedActor 저장
  (bind _ascharacter (cast `Character` OtherActor))
  (if (!= _ascharacter (`self.OwnerCharacter`))
    (`KismetArrayLibrary.Array_RemoveItem` (`self.OverlapedDamegedActors`) _ascharacter)))

(event `self.ReceiveTick`
  (params (DeltaSeconds :type "Float (single-precision)"))
  (`self.Particle`
    (:`then`
      (`|ExecutionSequence`
        (:`then_0`
          (`self.K2_SetActorLocation` (+ (`KismetMathLibrary.RotateAngleAxis` (`KismetMathLibrary.MakeVector` (`self.Distance`)) (`self.Angle`) (0.0 0.0 1.0)) (`self.K2_GetActorLocation` (`self.OwnerCharacter`)))))
        (:`then_1`
          (set `self.Angle` (+ (* (`self.Speed`) (`GameplayStatics.GetWorldDeltaSeconds`)) (`self.Angle`))))))
    (:`else`)))

(fn `Begin Do Action`
  (bind (_particlesystem _transform) (break `/Game/Structures/FEffect` (`.Effect_35_0FBB043C4820649C4A3CA79825DA37BA` (break `/Game/Structures/FAction` (`|GetArrayItem` (`self.ActionData`) 0)))))
  (`parent.Begin Do Action`)
  (bind _returnvalue (`GameplayStatics.SpawnEmitterAttached` _particlesystem (`self.Box`) "None" (.location _transform) (.rotation _transform) (.scale _transform)))
  (set `self.Particle` _returnvalue)
  (set `self.Angle` (`KismetMathLibrary.RandomFloatInRange` 0.0 360.0))
  (`PrimitiveComponent.SetCollisionEnabled` (`self.Box`) "QueryAndPhysics")
  (`KismetSystemLibrary.K2_SetTimerDelegate` (`|CreateDelegate` :!event `DestroyStorm`) (`self.Duration`))
  (`KismetSystemLibrary.K2_SetTimer` null "SendDamage" (`self.Interval`) true) ; if(Object == nullptr) Object = self
)

(fn `DestroyStorm`
  (`ActorComponent.K2_DestroyComponent` (`self.Particle`))
  (`PrimitiveComponent.SetCollisionEnabled` (`self.Box`) "NoCollision")
  (`KismetSystemLibrary.K2_ClearTimer` null "SendDamage") ; SendDamage의 타이머 초기화
)

(fn `DoAction`
  (`parent.DoAction`)
  (`self.Particle`
    (:`then`)
    (:`else`
      (bind _outobject (`/Game/MacroLibraries/ML_ObjectVerifier.VerifyImplementation` (`self.OwnerCharacter`) "/Game/Interfaces/IState.IState_C")
        (:`True`
          (bind _outresult (message `/Game/Interfaces/IState.IsState` _outobject "NewEnumerator0"))
          (if _outresult
            (message `/Game/Interfaces/IState.SetState` _outobject "NewEnumerator2")
            (`self.PlayAction` 0)))))))

(fn `EndDoAction`
  (`parent.EndDoAction`)
  (bind _outobject (`/Game/MacroLibraries/ML_ObjectVerifier.VerifyImplementation` (`self.OwnerCharacter`) "/Game/Interfaces/IState.IState_C")
    (:`True`
      (bind _outresult (message `/Game/Interfaces/IState.IsState` _outobject "NewEnumerator2"))
      (if _outresult
        (message `/Game/Interfaces/IState.SetState` _outobject "NewEnumerator0")
        (bind _outobject_2 (`/Game/MacroLibraries/ML_ObjectVerifier.VerifyImplementation` _outobject "/Game/Interfaces/IWeapon.IWeapon_C")
          (:`True`
            (message `/Game/Interfaces/IWeapon.SetWeaponMovable` _outobject_2 true)))))))

(event `DestroyStorm`)

(fn `SendDamage`
  ;[1 1 1] Overlap된 객체에 데미지 판정.
  (for _array_element (`self.OverlapedDamegedActors`)
    (`GameplayStatics.ApplyDamage` _array_element (`.Damage_24_F2016CD44BA9342BAF48A18FFE725F39` (break `/Game/Structures/FAction` (`|GetArrayItem` (`self.ActionData`)))) (`Pawn.GetController` (`self.OwnerCharacter`)) self)))

(fn `UserConstructionScript`
  (`parent.UserConstructionScript`))