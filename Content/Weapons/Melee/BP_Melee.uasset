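; BP_Melee is a melee weapon that plays combo attacks and damages actors its collision shapes overlap.
; DoAction starts an attack or queues a combo while its window is open; BeginDoAction advances the index, and EndDoAction resets it and owner state.
; Overlaps apply per-action damage, hit stop through global time dilation, camera shake, particles and sound.
; DamagedActors prevents repeat hits until collision is disabled.
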(event `self.ReceiveActorBeginOverlap`
  (params (OtherActor :type "Actor Object Reference"))
  (bind _returnvalue (`self.GetOwner`))
  (bind _hitstopdilation (`self.HitStopDilation`))
  (bind ((`Damage_24_F2016CD44BA9342BAF48A18FFE725F39` _damage) (`HitSTop_28_276970DB4567C344CA3A5D8BB25C2BA3` _hitstop) (`CameraShake_32_C08E2BE048322EC2E3930780389AD7EB` _camerashake) (`Effect_35_0FBB043C4820649C4A3CA79825DA37BA` _effect) (`Sound_38_A135D18547B7BDD68FF0DA9DBA7A9FF3` _sound)) (break `/Game/Structures/FAction` (`|GetArrayItem` (`self.ActionData`) (`self.Index`))))
  (bind (_particlesystem _transform) (break `/Game/Structures/FEffect` _effect))
  (if (!= (`self.GetOwner`) (`self.GetOwner` OtherActor))
    (if (!= OtherActor _returnvalue)
      (if (== (`KismetArrayLibrary.Array_Find` (`self.DamagedActors`) null) -1)
        ;[1 1 1] 데미지를 정상적으로 가했을 때만 실행.
        (bind _outobject (`/Game/MacroLibraries/ML_ObjectVerifier.VerifyValidity` (`self.GetInstigatorController` _returnvalue))
          (:`True`
            (`GameplayStatics.ApplyDamage` OtherActor (* _damage (`self.Damage`)) _outobject self)
            (`KismetArrayLibrary.Array_AddUnique` (`self.DamagedActors`) OtherActor)
            (if (!= 0.0 _hitstop)
              (`GameplayStatics.SetGlobalTimeDilation` _hitstopdilation)
              (`KismetSystemLibrary.K2_SetTimerDelegate` (`|CreateDelegate` :!event `RestoreTimeDilation`) (* _hitstopdilation _hitstop))
              (if (`KismetSystemLibrary.IsValidClass` _camerashake)
                (`PlayerCameraManager.StartCameraShake` :`self` (`PlayerController.PlayerCameraManager` (`GameplayStatics.GetPlayerController` 0)) :`ShakeClass` "/Game/Weapons/Melee/BP_Camera_Shake.BP_Camera_Shake_C")
                (bind _outobject_2 (`/Game/MacroLibraries/ML_ObjectVerifier.VerifyValidity` _particlesystem)
                  (:`True`
                    (`GameplayStatics.SpawnEmitterAtLocation` _outobject_2 (+ (`self.K2_GetActorLocation` OtherActor) (.location _transform)) (.rotation _transform) (.scale _transform))
                    (`GameplayStatics.SpawnSoundAtLocation` _sound (`self.K2_GetActorLocation` OtherActor) (struct) 1.0 1.0 0.0 null null)))))))))))

(fn `Begin Do Action`
  (`parent.Begin Do Action`)
  (if (`self.ComboTransfered`)
    (set `self.ComboTransfered` false)
    (`Character.StopAnimMontage` (`self.OwnerCharacter`) null)
    (bind _result (`/Engine/EditorBlueprintResources/StandardMacros.IncrementInt` (`self.Index`))
      (:`  `
        (`self.PlayAction` _result)))))

(fn `DoAction`
  (`parent.DoAction`)
  (if (`self.ComboEnabled`)
    (set `self.ComboEnabled` false)
    (set `self.ComboTransfered` true)
    (else
      (bind _outobject (`/Game/MacroLibraries/ML_ObjectVerifier.VerifyImplementation` (`self.OwnerCharacter`) "/Game/Interfaces/IState.IState_C")
        (:`True`
          (bind _outresult (message `/Game/Interfaces/IState.IsState` _outobject "NewEnumerator0"))
          (if _outresult
            (message `/Game/Interfaces/IState.SetState` _outobject "NewEnumerator2")
            (`self.PlayAction` (`self.Index`))))))))

(fn `EnableCollision`
  (params (`In Enabled` :type Boolean))
  (bind _returnvalue (`self.K2_GetComponentsByClass` "/Script/Engine.ShapeComponent"))
  (if `In Enabled`
    (for _array_element _returnvalue
      (`PrimitiveComponent.SetCollisionEnabled` _array_element "QueryAndPhysics"))
    (else
      (for _array_element_2 _returnvalue
        (`PrimitiveComponent.SetCollisionEnabled` _array_element_2 "NoCollision")
        (`KismetArrayLibrary.Array_Clear` (`self.DamagedActors`))))))

(fn `EndDoAction`
  (bind _ownercharacter (`self.OwnerCharacter`))
  (`parent.EndDoAction`)
  (set `self.Index` 0)
  ;[1 1 1] AnimMontage 비워놓으면 현재 재생중인 몽타주 끔.
  (`Character.StopAnimMontage` _ownercharacter null)
  (bind _outobject (`/Game/MacroLibraries/ML_ObjectVerifier.VerifyImplementation` _ownercharacter "/Game/Interfaces/IState.IState_C")
    (:`True`
      (message `/Game/Interfaces/IState.SetState` _outobject "NewEnumerator0")
      (bind _outobject_2 (`/Game/MacroLibraries/ML_ObjectVerifier.VerifyImplementation` _outobject "/Game/Interfaces/IWeapon.IWeapon_C")
        (:`True`
          (message `/Game/Interfaces/IWeapon.SetWeaponMovable` _outobject_2 true))))))

(fn `RestoreTimeDilation`
  (`GameplayStatics.SetGlobalTimeDilation` 1.0))

(fn `UserConstructionScript`
  (`parent.UserConstructionScript`))