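; BP_FireStorm is a weapon action that sends a fire storm, a particle effect with a collision box, orbiting its owner character.
; DoAction and EndDoAction check and set the owner's state through IState, then play the first action.
; BeginDoAction attaches the emitter from ActionData, randomizes the start angle and enables box collision.
; While the particle is valid, Tick repositions the actor by rotating a distance offset around the owner's Z axis.
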(event `self.ReceiveTick`
  (params (DeltaSeconds :type "Float (single-precision)"))
  (`self.Particle`
    (:`then`
      (`|ExecutionSequence`
        (:`then_0`
          (`self.K2_SetActorLocation` (+ (`KismetMathLibrary.RotateAngleAxis` (`KismetMathLibrary.MakeVector` (`self.Distance`)) (`self.Angle`) (0.0 0.0 1.0)) (`self.K2_GetActorLocation` (`self.OwnerCharacter`)))))
        (:`then_1`
          (set `self.Angle` (+ (* (`self.Speed`) (`GameplayStatics.GetWorldDeltaSeconds`)) (`self.Angle`))))))
    (:`else`)))

(fn `Begin Do Action`
  (bind (_particlesystem _transform) (break `/Game/Structures/FEffect` (`.Effect_35_0FBB043C4820649C4A3CA79825DA37BA` (break `/Game/Structures/FAction` (`|GetArrayItem` (`self.ActionData`) 0)))))
  (`parent.Begin Do Action`)
  (bind _returnvalue (`GameplayStatics.SpawnEmitterAttached` _particlesystem (`self.Box`) "None" (.location _transform) (.rotation _transform) (.scale _transform)))
  (set `self.Particle` _returnvalue)
  (set `self.Angle` (`KismetMathLibrary.RandomFloatInRange` 0.0 360.0))
  (`PrimitiveComponent.SetCollisionEnabled` (`self.Box`) "QueryAndPhysics"))

(fn `DoAction`
  (`parent.DoAction`)
  (bind _outobject (`/Game/MacroLibraries/ML_ObjectVerifier.VerifyImplementation` (`self.OwnerCharacter`) "/Game/Interfaces/IState.IState_C")
    (:`True`
      (bind _outresult (message `/Game/Interfaces/IState.IsState` _outobject "NewEnumerator0"))
      (if _outresult
        (message `/Game/Interfaces/IState.SetState` _outobject "NewEnumerator2")
        (`self.PlayAction` 0)))))

(fn `EndDoAction`
  (`parent.EndDoAction`)
  (bind _outobject (`/Game/MacroLibraries/ML_ObjectVerifier.VerifyImplementation` (`self.OwnerCharacter`) "/Game/Interfaces/IState.IState_C")
    (:`True`
      (bind _outresult (message `/Game/Interfaces/IState.IsState` _outobject "NewEnumerator0"))
      (if _outresult
        (message `/Game/Interfaces/IState.SetState` _outobject "NewEnumerator2")
        (`self.PlayAction` 0)))))

(fn `UserConstructionScript`
  (`parent.UserConstructionScript`))