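; Player character Blueprint that handles movement, camera look, dodging and switching between five weapon and skill types: one-hand, two-hand, teleport, firestorm and fireball.
; All weapons spawn at BeginPlay, and input forwards actions and skills to the equipped one.
; A state enum and Movable flag gate dodging, equipping and movement.
; Data tables supply equip and behavior montage data, plus per-weapon yaw lock applied when equipping ends.
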(event `self.ReceiveTick`
  (params (DeltaSeconds :type "Float (single-precision)"))
  (bind (_returnvalue_roll _returnvalue_pitch _returnvalue_yaw) (`KismetMathLibrary.BreakRotator` (`self.GetControlRotation`)))
  (`self.Is Movable`
    (:`True`
      (`self.AddMovementInput` (`KismetMathLibrary.Vector_Normal2D` (+ (* (`KismetMathLibrary.GetForwardVector` (`KismetMathLibrary.MakeRotator` 0.0 0.0 _returnvalue_yaw)) (`self.GetInputAxisValue`)) (* (`KismetMathLibrary.GetRightVector` (`KismetMathLibrary.MakeRotator` 0.0 0.0 _returnvalue_yaw)) (`self.GetInputAxisValue`))))))))

(event `self.ReceiveBeginPlay`
  (`/Game/MacroLibraries/ML_DataTableReader.ReadDataTable` (`self.BehaviorData`) "/Game/DataTables/DT_Behavior.DT_Behavior")
  (`/Game/MacroLibraries/ML_DataTableReader.ReadDataTable` (`self.EquipData`) "/Game/DataTables/DT_Equip.DT_Equip")
  (bind _returnvalue (`|SpawnActorFromClass` "/Game/Weapons/Melee/BP_OneHand.BP_OneHand_C" (`KismetMathLibrary.MakeTransform` (0.0 0.0 0.0)) "Undefined" "OverrideRootScale" self null))
  (set `self.OneHand` _returnvalue)
  (bind _returnvalue_2 (`|SpawnActorFromClass` "/Game/Weapons/Melee/BP_TwoHand.BP_TwoHand_C" (`KismetMathLibrary.MakeTransform` (0.0 0.0 0.0)) "Undefined" "OverrideRootScale" self null))
  (set `self.TwoHand` _returnvalue_2)
  (bind _returnvalue_3 (`|SpawnActorFromClass` "/Game/Weapons/Spell/BP_Teleport.BP_Teleport_C" (`KismetMathLibrary.MakeTransform` (0.0 0.0 -90.0)) "Undefined" "OverrideRootScale" self null))
  (set `self.Teleport` _returnvalue_3)
  (bind _returnvalue_4 (`|SpawnActorFromClass` "/Game/Weapons/Spell/BP_FireStorm.BP_FireStorm_C" (`KismetMathLibrary.MakeTransform` (0.0 0.0 0.0)) "Undefined" "OverrideRootScale" self null))
  (set `self.FireStorm` _returnvalue_4)
  (bind _returnvalue_5 (`|SpawnActorFromClass` "/Game/Weapons/Spell/BP_FireBall.BP_FireBall_C" (`KismetMathLibrary.MakeTransform` (0.0 0.0 0.0)) "Undefined" "OverrideRootScale" self null))
  (set `self.FireBall` _returnvalue_5))

(event `InputAxis|LookHorizontal`
  (params (AxisValue :type "Float (single-precision)"))
  (`self.Is Movable`
    (:`True`
      (`self.AddControllerYawInput` AxisValue))))

(event `InputAxis|LookVertical`
  (params (AxisValue :type "Float (single-precision)"))
  (`self.Is Movable`
    (:`True`
      (`self.AddControllerPitchInput` AxisValue))))

(event `InputAction|Act`
  (params (Key :type "Key Structure"))
  (:`Pressed`
    (bind _weapon (`self.Weapon`)
      (:`then`
        (`/Game/Weapons/BP_Weapon.DoAction` _weapon))
      (:`else`))))

(event `InputAction|Act2`
  (params (Key :type "Key Structure"))
  (:`Pressed`
    (bind _weapon (`self.Weapon`)
      (:`then`
        (`/Game/Weapons/BP_Weapon.DoPressedSkill` _weapon))
      (:`else`)))
  (:`Released`
    (bind _weapon_2 (`self.Weapon`)
      (:`then`
        (`/Game/Weapons/BP_Weapon.DoReleasedSkill` _weapon_2))
      (:`else`))))

(event `InputAction|OneHand`
  (params (Key :type "Key Structure"))
  (:`Pressed`
    (`self.ChangeWeapon` (`self.OneHand`))))

(event `InputAction|Dodge`
  (params (Key :type "Key Structure"))
  (:`Pressed`
    (`self.Is Movable`
      (:`True`
        (`self.Begin Dodge`)))))

(event `InputAction|TwoHand`
  (params (Key :type "Key Structure"))
  (:`Pressed`
    (`self.ChangeWeapon` (`self.TwoHand`))))

(event `InputAction|Teleport`
  (params (Key :type "Key Structure"))
  (:`Pressed`
    (`self.ChangeWeapon` (`self.Teleport`))))

(event `InputAction|FireStorm`
  (params (Key :type "Key Structure"))
  (:`Pressed`
    (`self.ChangeWeapon` (`self.FireStorm`))))

(event `InputAction|FireBall`
  (params (Key :type "Key Structure"))
  (:`Pressed`
    (`self.ChangeWeapon` (`self.FireBall`))))

(fn `Begin Dodge`
  (bind _outresult (`self.IsState` "NewEnumerator0"))
  (if _outresult
    (`/Game/MacroLibraries/ML_ObjectVerifier.VerifyValidity` (`self.Weapon`)
      (:`True`
        (set `self.Movable` false)
        (set `self.bUseControllerRotationYaw` false)
        (`self.K2_SetActorRotation` (`KismetMathLibrary.MakeRotFromX` (* (`KismetMathLibrary.GreaterGreater_VectorRotator` (`KismetMathLibrary.MakeVector` (`self.GetInputAxisValue`) (`self.GetInputAxisValue`)) (`self.K2_GetActorRotation`)) (+ 0.5 (`self.GetInputAxisValue`)))))
        (if (> 0.0 (`self.GetInputAxisValue`))
          (`self.SetState` "NewEnumerator4")
          (else
            (`self.SetState` "NewEnumerator3")))
        (`/Game/FunctionLibraries/FL_MontagePlayer.PlayBehaviorMontage` self (`self.StateType`) (`self.BehaviorData`))))))

(fn `ChangeWeapon`
  (params (InWeapon :type "/Game/Weapons/BP_Weapon Object Reference"))
  (returns (OutResult :type Boolean))
  (bind _outresult (`self.IsState` "NewEnumerator0"))
  (if _outresult
    (bind _weapon (`self.Weapon`)
      (:`then`
        (if (== (`local.InWeapon`) _weapon)
          (`self.Unequip`)
          (else
            (`self.Unequip`)
            (bind _output_get (set `self.Weapon` (`local.InWeapon`) :!label _label))
            (`self.SetState` "NewEnumerator1")
            (bind _outresult_2 (`/Game/FunctionLibraries/FL_MontagePlayer.PlayEquipMontage` self (`/Game/Weapons/BP_Weapon.WeaponType` _output_get) (`self.EquipData`)))
            (if _outresult_2
              (return true)
              (else
                (`self.WeaponBeginEquip`)
                (`self.WeaponEndEquip`)
                (return false))))))
      (:`else`
        (goto _label))))
  (return false))

(fn `End Dodge`
  (set `self.bUseControllerRotationYaw` true)
  (set `self.Movable` true)
  (`self.SetState` "NewEnumerator0"))

(fn `GetWeapon`
  (returns (OutWeapon :type "/Game/Weapons/BP_Weapon Object Reference"))
  (return (`self.Weapon`)))

(fn `IsState`
  (params (InState :type "/Game/Enumerations/EStateType Enum" :default "NewEnumerator0"))
  (returns (OutResult :type Boolean))
  (return (`|EnumEquality` InState (`self.StateType`))))

(fn `SetState`
  (params (InState :type "/Game/Enumerations/EStateType Enum" :default "NewEnumerator0"))
  (returns (OutState :type "/Game/Enumerations/EStateType Enum"))
  (bind _output_get (set `self.StateType` InState))
  (return _output_get))

(fn `SetWeaponMovable`
  (params (InMovable :type Boolean))
  (returns (OutResult :type Boolean))
  (bind _output_get (set `self.Movable` InMovable))
  (return _output_get))

(fn `Unequip`
  (bind _outresult (`self.IsState` "NewEnumerator0"))
  (if _outresult
    (`/Game/Weapons/BP_Weapon.Unequip` (`self.Weapon`))
    (set `self.Weapon` null)
    (set `self.bUseControllerRotationYaw` false)))

(fn `UserConstructionScript`)

(fn `WeaponBeginEquip`
  (returns (OutResult :type Boolean))
  (bind _weapon (`self.Weapon`)
    (:`then`
      (`/Game/Weapons/BP_Weapon.BeginEquip` _weapon)
      (return false))
    (:`else`)))

(fn `WeaponEndEquip`
  (returns (OutResult :type Boolean))
  (bind _weapon (`self.Weapon`))
  (`/Game/Weapons/BP_Weapon.EndEquip` _weapon)
  (for _array_element (`self.EquipData`)
    (if (`|EnumEquality` (break `/Game/Structures/FEquip` _array_element) (`/Game/Weapons/BP_Weapon.WeaponType` _weapon))
      (set `self.bUseControllerRotationYaw` (`.LockedLook_16_8549711643B7F514AD153E944209C10D` (break `/Game/Structures/FEquip` _array_element)))
      (`self.SetState` "NewEnumerator0")
      (return false))))